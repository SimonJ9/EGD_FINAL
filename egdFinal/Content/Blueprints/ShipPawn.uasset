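; Drivable ship pawn that a Driver character can leave with E, handing possession back to that character.
; Forward and turn inputs go through server events that offset and yaw the ship on authority.
; Server Tick pins the Driver to Spot, prints on nearing the Destination, and scans EnemyMinion states to control AmbientSound actors.
; Both sound branches only stop audio, as Play is disconnected; TakeDamage just lowers HP to zero minimum.
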(event `self.ReceiveBeginPlay`
  ;[1 1 1] Set Speed
  (`/Engine/EditorBlueprintResources/ActorMacros.Switch Has Authority`
    (:`Authority`
      (set `self.speed` 1300.0)
      (`self.AssignDestination`)
      (bind _outactors (`GameplayStatics.GetAllActorsOfClass` "/Script/Engine.AmbientSound"))
      (for _array_element _outactors
        (`AudioComponent.Stop` (`AmbientSound.AudioComponent` _array_element))))))

(event `AddRotateServer`
  (params (Axis :type "Float (double-precision)") (deltaTime :type "Float (double-precision)"))
  ;[1 1 1] Add Actor Local Rotation
  (`self.UpdateRotation` Axis deltaTime))

(event `InputAxis|right`
  (params (AxisValue :type "Float (single-precision)"))
  ;[1 1 1] Add Actor Local Rotation
  (`self.AddRotateServer` AxisValue (stale `self.ReceiveTick` DeltaSeconds)))

(event `self.ReceiveTick`
  (params (DeltaSeconds :type "Float (single-precision)"))
  (`/Engine/EditorBlueprintResources/ActorMacros.Switch Has Authority`
    (:`Authority`
      (`self.NewFunction_0`)
      ;[1 1 1] Update Drive Location
      (`self.UpdateDriverLoc`)
      ;[1 1 1] On Get To Destination
      (bind _isnear (`self.IsNearToDes` 2000.0))
      (if _isnear
        (`self.OnReachDestination`))
      (`self.NewFunction_1`))))

(event `Key|E`
  (params (Key :type "Key Structure"))
  ;[1 1 1] Get Off Vehicle
  (:`Pressed`
    (if (not (== (`self.Driver`) null))
      (`/Engine/EditorBlueprintResources/ActorMacros.Switch Has Authority`
        (:`Authority`
          (`self.GetOffVehicle` :!label _label))
        (:`Remote`
          (`self.GetOffVehicleServer`))))))

(event `InputAxis|forward`
  (params (AxisValue :type "Float (single-precision)"))
  ;[1 1 1] Add Movement Input
  (`self.AddMovementServer` AxisValue (stale `self.ReceiveTick` DeltaSeconds)))

(event `GetOffVehicleServer`
  ;[1 1 1] Get Off Vehicle
  (goto _label))

(event `AddMovementServer`
  (params (Axis :type "Float (double-precision)") (deltaTime :type "Float (double-precision)"))
  ;[1 1 1] Add Movement Input
  (`self.UpdateMovement` Axis deltaTime))

(event `GetOffVehicle`
  (bind _driver (`self.Driver`))
  ;[1 1 1] Get Off Vehicle
  (`/Engine/EditorBlueprintResources/ActorMacros.Switch Has Authority`
    (:`Authority`
      (`Controller.Possess` (`self.GetController`) _driver)
      (set `/Game/Blueprints/PlayerController.Incar` false _driver)
      (set `self.Driver` null))))

(fn `AssignDestination`
  (bind _outactors (`GameplayStatics.GetAllActorsOfClass` "/Game/Destination_Blueprint.Destination_Blueprint_C"))
  (for _array_element _outactors
    (set `self.Destination` _array_element)
    (break)))

(fn `IsNearToDes`
  (params (distance :type "Float (double-precision)"))
  (returns (isNear :type Boolean))
  (return (< (`self.GetDistanceTo` (`self.Destination`)) distance)))

(fn `NewFunction_0`)

(fn `NewFunction_1`
  (bind _outactors (`GameplayStatics.GetAllActorsOfClass` "/Game/Blueprints/EnemyMinion.EnemyMinion_C"))
  (set `self.noneleft` true)
  (for _array_element _outactors
    (if (== (`/Game/Blueprints/EnemyMinion.State` _array_element) 0)
      (set `self.noneleft` false)))
  (if (`self.noneleft`)
    (bind _outactors_2 (`GameplayStatics.GetAllActorsOfClass` "/Script/Engine.AmbientSound"))
    (for _array_element_2 _outactors_2
      (`AudioComponent.Stop` (`AmbientSound.AudioComponent` _array_element_2)))
    (else
      (bind _outactors_3 (`GameplayStatics.GetAllActorsOfClass` "/Script/Engine.AmbientSound"))
      (for _array_element_3 _outactors_3
        (bind _audiocomponent (`AmbientSound.AudioComponent` _array_element_3))
        (if (not (`AudioComponent.IsPlaying` _audiocomponent))
          (`AudioComponent.Stop` _audiocomponent))))))

(fn `OnReachDestination`
  (`KismetSystemLibrary.PrintString` "Reach Destination"))

(fn `TakeDamage`
  (params (amount :type "Float (double-precision)"))
  (set `self.HP` (`KismetMathLibrary.FMax` (- (`self.HP`) amount))))

(fn `UpdateDriverLoc`
  (bind _driver (`self.Driver`))
  (if (not (== _driver null))
    (`self.K2_SetActorLocation` _driver (`self.K2_GetActorLocation` (`self.Spot`)) false true)))

(fn `UpdateMovement`
  (params (Axis :type "Float (double-precision)") (deltaTime :type "Float (double-precision)"))
  (`/Engine/EditorBlueprintResources/ActorMacros.Switch Has Authority`
    (:`Authority`
      (bind _output_get (set `self.Forward` (`KismetMathLibrary.GetForwardVector` (`KismetMathLibrary.MakeRotator` 0.0 0.0 (.yaw (`self.K2_GetActorRotation`))))))
      (bind _output_get_2 (set `self.speedA` (* Axis (`self.speed`) deltaTime)))
      (`self.K2_AddActorWorldOffset` self (* _output_get _output_get_2) false false))))

(fn `UpdateRotation`
  (params (Axis :type "Float (double-precision)") (deltaTime :type "Float (double-precision)"))
  (`/Engine/EditorBlueprintResources/ActorMacros.Switch Has Authority`
    (:`Authority`
      (bind _output_get (set `self.RotateRight` (`KismetMathLibrary.MakeRotator` 0.0 0.0 (* deltaTime Axis 10.0))))
      (`self.K2_AddActorLocalRotation` self _output_get false false))))

(fn `UserConstructionScript`)