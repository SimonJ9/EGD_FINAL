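; A hint actor that keeps a sparks particle hovering above itself and, when GiveAHint is called, sends it toward the destination as a directional clue.
; On BeginPlay, the authority stores the first Destination_Blueprint actor found.
; GiveAHint promotes the idle emitter to the moving one.
; Tick drifts it upward and horizontally toward the destination with growing speed, destroys it after a timeout, then spawns a replacement.
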(event `self.ReceiveBeginPlay`
  (`/Engine/EditorBlueprintResources/ActorMacros.Switch Has Authority`
    (:`Authority`
      (bind _outactors (`GameplayStatics.GetAllActorsOfClass` "/Game/Destination_Blueprint.Destination_Blueprint_C"))
      (for _array_element _outactors
        (set `self.Destination` _array_element)
        (break)))))

(event `self.ReceiveTick`
  (params (DeltaSeconds :type "Float (single-precision)"))
  (bind _particle (`self.Particle`))
  (bind _timer (`self.Timer`))
  (bind _returnvalue (`SceneComponent.K2_GetComponentLocation` _particle))
  (bind _returnvalue_2 (* (`self.Timer`) 25.0))
  ;[1 1 1] Move Particle
  (if (!= _particle null)
    (`SceneComponent.K2_SetWorldLocation` _particle (+ _returnvalue (* (+ (`KismetMathLibrary.Normal` (* (- (`self.K2_GetActorLocation` (`self.Destination`)) _returnvalue) (1.0 1.0 0.0))) (0.0 0.0 1.0)) (* (`KismetMathLibrary.MakeVector` _returnvalue_2 _returnvalue_2 100.0) DeltaSeconds))) false false)
    (if (>= _timer 15.0)
      (set `self.Timer` 0.0)
      (`ActorComponent.K2_DestroyComponent` (`self.Particle`))
      (set `self.Particle` null)
      (else
        (set `self.Timer` (+ _timer DeltaSeconds))))
    (elif (== (`self.StaticParticle`) null)
      (bind _returnvalue_3 (`GameplayStatics.SpawnEmitterAtLocation` "/Game/StarterContent/Particles/P_Sparks.P_Sparks" (+ (`self.K2_GetActorLocation`) (0.0 0.0 150.0))))
      (set `self.StaticParticle` _returnvalue_3))))

(fn `GiveAHint`
  (bind _staticparticle (`self.StaticParticle`))
  (if (== (`self.Particle`) null)
    (if (!= _staticparticle null)
      (set `self.Particle` _staticparticle)
      (set `self.StaticParticle` null))))

(fn `UserConstructionScript`)