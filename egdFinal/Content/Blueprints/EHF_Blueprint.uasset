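; Height fog actor that adjusts the fog start distance based on the player's relation to a vehicle.
; Each tick, when Player and Vehicle references are valid, it casts the player to PlayerControllerT and reads its Incar flag.
; In the car, fog starts at a fixed far distance; otherwise that distance shrinks by the player-to-vehicle distance, clamped at zero, so fog closes in as the player moves away.
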(event `self.ReceiveBeginPlay`)

(event `self.ReceiveTick`
  (params (DeltaSeconds :type "Float (single-precision)"))
  (bind _exponentialheightfog (`self.ExponentialHeightFog`))
  (bind _player (`self.Player`))
  (bind _vehicle (`self.Vehicle`))
  ;[1 1 1] Handle fog effect
  (if (!= _player null)
    (if (!= _vehicle null)
      (bind _asplayer_controller_t (cast `/Game/Blueprints/PlayerControllerT` (`self.Player`)))
      (if (`/Game/Blueprints/PlayerControllerT.Incar` _asplayer_controller_t)
        (`ExponentialHeightFogComponent.SetStartDistance` _exponentialheightfog 8500.0)
        (else
          (`ExponentialHeightFogComponent.SetStartDistance` _exponentialheightfog (`KismetMathLibrary.FMax` (- 8500.0 (`self.GetDistanceTo` _player _vehicle)))))))))

(fn `UserConstructionScript`)