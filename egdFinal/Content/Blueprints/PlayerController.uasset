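; On-foot player character, despite the PlayerController name, tied to the level's ShipPawn, with movement, an HP widget and EHF setup.
; Left click spawns Sphere_Blueprint projectiles aimed by camera trace; E possesses the overlapped, driverless ship or otherwise triggers hint objects.
; The authority drains HP when the player strays too far from the ship.
; At zero HP it damages the ship as a penalty and, depending on the result, respawns the player nearby.
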(event `self.ReceiveBeginPlay`
  (`self.Initialize`)
  (bind _returnvalue (`|CreateWidget` "/Game/hpbar.hpbar_C"))
  ;[1 1 1] Camera rotation not affect character
  (bind _output_get (set `self.hpref` _returnvalue))
  (`UserWidget.AddToViewport` _output_get 0)
  (set `self.bUseControllerRotationPitch` false)
  (set `self.bUseControllerRotationRoll` false)
  (set `self.bUseControllerRotationYaw` true)
  (if (`self.IsLocallyControlled`)
    (if (== (`self.EHF`) null)
      (bind _outactors (`GameplayStatics.GetAllActorsOfClass` "/Game/Blueprints/EHF_Blueprint.EHF_Blueprint_C"))
      (for _array_element _outactors
        (bind _output_get_2 (set `self.EHF` _array_element))
        (break))
      (set `/Game/Blueprints/EHF_Blueprint.Player` self _output_get_2)
      (set `/Game/Blueprints/EHF_Blueprint.Vehicle` (`self.Vehicle`) _output_get_2))))

(event `InputAxis|rotate_horizontal`
  (params (AxisValue :type "Float (single-precision)"))
  ;[1 1 1] rotation and jump
  (`self.AddControllerYawInput` AxisValue))

(event `InputAction|Jump`
  (params (Key :type "Key Structure"))
  ;[1 1 1] rotation and jump
  (:`Pressed`
    (`self.Jump`))
  (:`Released`
    (`self.StopJumping`)))

(event `UpdateEHFServer`
  ;[1 1 1] Take Damage When Too Far Away From Ship
)

(event `UpdateEHF`
  ;[1 1 1] Take Damage When Too Far Away From Ship
)

(event `InputAxis|look_up_down`
  (params (AxisValue :type "Float (single-precision)"))
  ;[1 1 1] rotation and jump
  (`self.AddControllerPitchInput` AxisValue))

(event `self.ReceiveTick`
  (params (DeltaSeconds :type "Float (single-precision)"))
  (`/Engine/EditorBlueprintResources/ActorMacros.Switch Has Authority`
    (:`Authority`
      ;[1 1 1] Take Damage When Too Far Away From Ship
      (if (> (`self.GetDistanceTo` (`self.Vehicle`)) 8500.0)
        (`self.TakeDemage` (* DeltaSeconds 5.0))))))

(event `Key|LeftMouseButton`
  (params (Key :type "Key Structure"))
  (bind _playercamera (`self.PlayerCamera`))
  (:`Pressed`
    (`self.rekt` (`KismetMathLibrary.MakeTransform` (`SceneComponent.K2_GetComponentLocation` (`self.Sphere`)) (`SceneComponent.K2_GetComponentRotation` _playercamera)) _playercamera)))

(event `rekt`
  (params (trans :type "Transform Structure") (actor :type "SceneComponent Object Reference"))
  (`self.shoot` trans actor))

(event `ActivateHintObject`
  (params (HintObj :type "/Game/Blueprints/HintObject_Blueprint Object Reference"))
  ;[1 1 1] Activate Hint Object
  (`KismetSystemLibrary.PrintString` (`KismetSystemLibrary.GetDisplayName` HintObj))
  (`/Game/Blueprints/HintObject_Blueprint.GiveAHint` HintObj))

(event `InputAxis|forward`
  (params (AxisValue :type "Float (single-precision)"))
  ;[1 1 1] Horozontal movement
  (`self.AddMovementInput` (`KismetMathLibrary.GetForwardVector` (`KismetMathLibrary.MakeRotator` 0.0 0.0 (.yaw (`self.GetControlRotation`)))) AxisValue))

(event `ActivateHintObject_Server`
  (params (HintObj :type "/Game/Blueprints/HintObject_Blueprint Object Reference"))
  ;[1 1 1] Activate Hint Object
  (`self.ActivateHintObject` HintObj))

(event `InputAxis|right`
  (params (AxisValue :type "Float (single-precision)"))
  ;[1 1 1] Horozontal movement
  (`self.AddMovementInput` (`KismetMathLibrary.GetRightVector` (`KismetMathLibrary.MakeRotator` 0.0 0.0 (.yaw (`self.GetControlRotation`)))) AxisValue))

(event `Key|E`
  (params (Key :type "Key Structure"))
  ;[1 1 1] Get On Vehicle
  (:`Pressed`
    (`KismetSystemLibrary.PrintString` "Pressing E")
    (if (`self.IsOverlappingActor` (`self.Vehicle`))
      (`KismetSystemLibrary.PrintString` "Is overlapping")
      (if (`self.Incar`)
        _
        (elif (== (`/Game/Blueprints/ShipPawn.Driver` (`self.Vehicle`)) null)
          (`KismetSystemLibrary.PrintString` "GEt into car")
          (`/Engine/EditorBlueprintResources/ActorMacros.Switch Has Authority`
            (:`Authority`
              (`self.GetOnVehicle` :!label _label))
            (:`Remote`
              (`self.GetOnVehicleServer`)))))
      (else
        ;[1 1 1] Activate Hint Object
        (for _array_element (`self.GetOverlappingActors` "/Game/Blueprints/HintObject_Blueprint.HintObject_Blueprint_C")
          (bind _ashint_object_blueprint (cast `/Game/Blueprints/HintObject_Blueprint` _array_element))
          (`self.ActivateHintObject_Server` _ashint_object_blueprint)
          (break))))))

(event `GetOnVehicle`
  (bind _driver (`/Game/Blueprints/ShipPawn.Driver` (`self.Vehicle`)))
  (bind _returnvalue (`self.GetController` _driver))
  ;[1 1 1] Get On Vehicle
  (`KismetSystemLibrary.PrintString` "Get On Vehicle")
  (if (== _driver null)
    (bind _output_get (set `/Game/Blueprints/ShipPawn.Driver` self (`self.Vehicle`)))
    (set `/Game/Blueprints/PlayerController.Incar` true _output_get)
    (`KismetSystemLibrary.PrintString` (`KismetSystemLibrary.GetDisplayName` _driver))
    (if (not (== _returnvalue null))
      (`Controller.Possess` _returnvalue (`self.Vehicle`)))))

(event `GetOnVehicleServer`
  ;[1 1 1] Get On Vehicle
  (goto _label))

(event `Key|Slash`
  (params (Key :type "Key Structure"))
  (:`Pressed`
    (set `self.HP` (- (`self.HP`) 1.0))))

(fn `Initialize`
  (`/Engine/EditorBlueprintResources/ActorMacros.Switch Has Authority`
    (:`Authority`
      (set `self.RespawnPenalty` 10.0))))

(fn `shoot`
  (params (trans :type "Transform Structure") (actor :type "SceneComponent Object Reference"))
  (bind _returnvalue (`SceneComponent.K2_GetComponentLocation` actor))
  (bind _returnvalue_2 (+ _returnvalue (* (`KismetMathLibrary.GetForwardVector` (`SceneComponent.K2_GetComponentRotation` actor)) 1500.0)))
  (bind (_outhit _returnvalue_3) (`KismetSystemLibrary.LineTraceSingle` _returnvalue _returnvalue_2 "TraceTypeQuery2" false (`|MakeArray` self :!type "Actor Object Reference")))
  (if _returnvalue_3
    (set `self.hitlocation` (`.Location` (`GameplayStatics.BreakHitResult` _outhit)))
    (else
      (set `self.hitlocation` _returnvalue_2)))
  (`|SpawnActorFromClass` "/Game/Sphere_Blueprint.Sphere_Blueprint_C" (`KismetMathLibrary.MakeTransform` (.location trans) (`KismetMathLibrary.FindLookAtRotation` _returnvalue (`self.hitlocation`)) (.scale trans)) "AlwaysSpawn" "OverrideRootScale" null null))

(fn `TakeDemage`
  (params (Demage :type "Float (double-precision)"))
  (`/Engine/EditorBlueprintResources/ActorMacros.Switch Has Authority`
    (:`Authority`
      (bind _output_get (set `self.HP` (`KismetMathLibrary.FMax` (- (`self.HP`) Demage))))
      (`KismetSystemLibrary.PrintString` (`KismetStringLibrary.Conv_DoubleToString` _output_get))
      (if (<= _output_get 0.0)
        (`self.TryToRespawn`)))))

(fn `TryToRespawn`
  (`/Engine/EditorBlueprintResources/ActorMacros.Switch Has Authority`
    (:`Authority`
      (bind _iszero (`/Game/Blueprints/ShipPawn.TakeDamage` (`self.Vehicle`) (`self.RespawnPenalty`)))
      (if (not _iszero)
        (set `self.HP` 100.0)
        (`self.K2_SetActorLocation` (+ (* (`KismetMathLibrary.Normal` (`KismetMathLibrary.MakeVector` (`KismetMathLibrary.RandomFloat`) (`KismetMathLibrary.RandomFloat`) 0.0)) 3000.0) (0.0 0.0 1500.0) (`self.K2_GetActorLocation` (`self.Vehicle`))))))))

(fn `UserConstructionScript`
  (`/Engine/EditorBlueprintResources/ActorMacros.Switch Has Authority`
    (:`Authority`
      _)
    (:`Remote`
      _))
  (bind _outactors (`GameplayStatics.GetAllActorsOfClass` "/Game/Blueprints/ShipPawn.ShipPawn_C"))
  (for _array_element _outactors
    (bind _asship_pawn (cast `/Game/Blueprints/ShipPawn` _array_element))
    (set `self.Vehicle` _asship_pawn))
  (set `self.Incar` false))