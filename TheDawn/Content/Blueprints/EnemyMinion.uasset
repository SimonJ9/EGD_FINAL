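; Enemy minion that spins as it chases the ShipPawn and explodes on overlapping it or a PlayerControllerT, dealing damage.
; Movement, spin and overlap attacks run on authority from Tick, using straight offsets without sweep.
; It switches between chasing and returning to spawn by the ship's distance from that origin, with separate leave and re-engage thresholds.
; TakeDamage drains health; death or explosion plays a random hit sound and destroys the actor.
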(event `self.ReceiveBeginPlay`
  (`/Engine/EditorBlueprintResources/ActorMacros.Switch Has Authority`
    (:`Authority`
      (set `self.clockwise` (`KismetMathLibrary.RandomBool`))
      (set `self.speed` 700.0)
      (bind _outactors (`GameplayStatics.GetAllActorsOfClass` "/Game/Blueprints/ShipPawn.ShipPawn_C"))
      (for _array_element _outactors
        (set `self.shipref` _array_element)
        (break))
      (set `self.maxChaseDistance` (+ (* (`KismetMathLibrary.RandomFloat`) 500.0) 12500.0))
      (set `self.maxAttractDistance` 7500.0)
      (set `self.spawnOrigin` (`self.K2_GetActorLocation`))
      (set `self.Health` 100.0)
      (set `self.Damage` 20.0))))

(event `PlayDeathSoundServer`
  (`self.PlayDeathSound`))

(event `self.ReceiveTick`
  (params (DeltaSeconds :type "Float (single-precision)"))
  (bind _state (`self.State`))
  (`self.Attack`)
  (if (== _state 0)
    (`self.ChaseToShip` DeltaSeconds)
    (elif (== _state 1)
      (`self.BackToOrigin` DeltaSeconds))))

(event `PlayDeathSound`
  (bind _returnvalue (`self.K2_GetActorLocation`))
  (if (`KismetMathLibrary.RandomBool`)
    (`GameplayStatics.PlaySoundAtLocation` "/Game/Sound/Hit1.Hit1" _returnvalue)
    (else
      (`GameplayStatics.PlaySoundAtLocation` "/Game/Sound/Hit2.Hit2" _returnvalue))))

(fn `Attack`
  (bind _overlappingactors (`self.GetOverlappingActors` null))
  (bind _damage (`self.Damage`))
  (`/Engine/EditorBlueprintResources/ActorMacros.Switch Has Authority`
    (:`Authority`
      (if (!= (`KismetArrayLibrary.Array_Length` _overlappingactors) 0)
        (for _array_element _overlappingactors
          (bind _asship_pawn (cast `/Game/Blueprints/ShipPawn` _array_element)
            (:`then`
              (`/Game/Blueprints/ShipPawn.TakeDamage` _asship_pawn _damage))
            (:`CastFailed`
              (bind _asplayer_controller_t (cast `/Game/Blueprints/PlayerControllerT` _array_element))
              (`/Game/Blueprints/PlayerControllerT.TakeDemage` _asplayer_controller_t _damage)))
          (`self.Explode`))))))

(fn `BackToOrigin`
  (params (deltaTIme :type "Float (double-precision)"))
  (bind _returnvalue (* (`self.speed`) deltaTIme))
  (`/Engine/EditorBlueprintResources/ActorMacros.Switch Has Authority`
    (:`Authority`
      (`self.K2_AddActorWorldOffset` self (* (`KismetMathLibrary.Normal` (- (`self.spawnOrigin`) (`self.K2_GetActorLocation`))) _returnvalue) false false)
      (if (`self.clockwise`)
        (`self.K2_AddActorLocalRotation` (`KismetMathLibrary.MakeRotator` 0.0 0.0 _returnvalue))
        (else
          (`self.K2_AddActorLocalRotation` (`KismetMathLibrary.MakeRotator` 0.0 0.0 (* _returnvalue -1.0)))))
      (if (<= (`KismetMathLibrary.VSize` (- (`self.spawnOrigin`) (`self.K2_GetActorLocation` (`self.shipref`)))) (`self.maxAttractDistance`))
        (set `self.State` 0)))))

(fn `ChaseToShip`
  (params (B :type "Float (double-precision)"))
  (bind _returnvalue (* (`self.speed`) B))
  (`/Engine/EditorBlueprintResources/ActorMacros.Switch Has Authority`
    (:`Authority`
      (`self.K2_AddActorWorldOffset` self (* (`KismetMathLibrary.Normal` (- (`SceneComponent.K2_GetComponentLocation` (`/Game/Blueprints/ShipPawn.Box` (`self.shipref`))) (`self.K2_GetActorLocation`))) _returnvalue) false false)
      (if (`self.clockwise`)
        (`self.K2_AddActorLocalRotation` (`KismetMathLibrary.MakeRotator` 0.0 0.0 _returnvalue))
        (else
          (`self.K2_AddActorLocalRotation` (`KismetMathLibrary.MakeRotator` 0.0 0.0 (* _returnvalue -1.0)))))
      (if (>= (`KismetMathLibrary.VSize` (- (`self.spawnOrigin`) (`self.K2_GetActorLocation` (`self.shipref`)))) (`self.maxChaseDistance`))
        (set `self.State` 1)))))

(fn `Explode`
  (`KismetSystemLibrary.PrintString` "Explode")
  (`self.PlayDeathSoundServer`)
  (`self.K2_DestroyActor`))

(fn `TakeDamage`
  (params (Amount :type "Float (double-precision)"))
  (bind _output_get (set `self.Health` (`KismetMathLibrary.FMax` (- (`self.Health`) Amount))))
  (if (<= _output_get 0.0)
    (`self.PlayDeathSoundServer`)
    (`self.K2_DestroyActor`)))

(fn `UserConstructionScript`)