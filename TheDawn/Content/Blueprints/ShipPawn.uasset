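; Drivable ship pawn for a networked game, won by reaching a destination and lost when its HP hits zero.
; Axis inputs feed server events that offset and rotate the actor under authority checks and scale the engine sound.
; Server Tick pins the Driver to Spot, tests destination distance and pushes overlapping players away.
; Keys handle exiting by repossessing the Driver, a helper widget, and post-game level restart via servertravel.
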(event `Key|Tab`
  (params (Key :type "Key Structure"))
  ;[1 1 1] Show Helper UI
  (:`Pressed`
    (bind _returnvalue (`|CreateWidget` "/Game/sUI.sUI_C"))
    (`UserWidget.AddToViewport` _returnvalue 0))
  (:`Released`
    (`Widget.RemoveFromParent` _returnvalue)))

(event `HideLostUI`
  ;[1 1 1] Hide Win/Lost UI
)

(event `HideWinUI`
  ;[1 1 1] Hide Win/Lost UI
)

(event `self.ReceiveBeginPlay`
  ;[1 1 1] Set Speed
  (`self.ClearUI`)
  (set `self.NeedUIFlag` true)
  (`/Engine/EditorBlueprintResources/ActorMacros.Switch Has Authority`
    (:`Authority`
      (set `self.speed` 1300.0)
      (`self.AssignDestination`)
      (set `self.isGameNotOver` true))))

(event `DisplayLostUI`
  ;[1 1 1] Show Win/Lost UI
  (if (`self.NeedUIFlag`)
    (set `self.NeedUIFlag` false)
    (bind _returnvalue (`|CreateWidget` "/Game/LostUI.LostUI_C"))
    (`UserWidget.AddToViewport` _returnvalue 0)))

(event `Key|R`
  (params (Key :type "Key Structure"))
  ;[1 1 1] Restart Game
  (:`Pressed`
    (if (not (`self.isGameNotOver`))
      (`self.RestartGameServer`))))

(event `PlayMovingSound`
  (params (Volume :type "Float (double-precision)"))
  (`AudioComponent.SetVolumeMultiplier` (`self.ShipMovingSound`) Volume))

(event `RestartGameServer`
  ;[1 1 1] Restart Game
  (`KismetSystemLibrary.ExecuteConsoleCommand` "servertravel Level1"))

(event `DisplayWinUI`
  ;[1 1 1] Show Win/Lost UI
  (if (`self.NeedUIFlag`)
    (set `self.NeedUIFlag` false)
    (bind _returnvalue (`|CreateWidget` "/Game/WinUI.WinUI_C"))
    (`UserWidget.AddToViewport` _returnvalue 0)))

(event `AddRotateServer`
  (params (Axis :type "Float (double-precision)") (deltaTime :type "Float (double-precision)"))
  ;[1 1 1] Add Actor Local Rotation
  (`self.UpdateRotation` Axis deltaTime)
  (`self.PlayMovingSound` (`KismetMathLibrary.FMin` (+ (`KismetMathLibrary.Abs` Axis) (`KismetMathLibrary.Abs` (stale `AddMovementServer` Axis))) 1.0)))

(event `OnReachDestinationSever`)

(event `InputAxis|right`
  (params (AxisValue :type "Float (single-precision)"))
  ;[1 1 1] Add Actor Local Rotation
  (if (`self.isGameNotOver`)
    (`self.AddRotateServer` AxisValue (stale `self.ReceiveTick` DeltaSeconds))))

(event `self.ReceiveTick`
  (params (DeltaSeconds :type "Float (single-precision)"))
  (`/Engine/EditorBlueprintResources/ActorMacros.Switch Has Authority`
    (:`Authority`
      ;[1 1 1] Update Drive Location
      (`self.UpdateDriverLoc`)
      ;[1 1 1] On Get To Destination
      (bind _isnear (`self.IsNearToDes` 2000.0))
      (if _isnear
        (`self.OnReachDestination`))
      (`self.RepelPlayer` DeltaSeconds (stale `InputAxis|forward` AxisValue)))))

(event `InputAxis|forward`
  (params (AxisValue :type "Float (single-precision)"))
  ;[1 1 1] Add Movement Input
  (if (`self.isGameNotOver`)
    (`self.AddMovementServer` AxisValue (stale `self.ReceiveTick` DeltaSeconds))))

(event `Key|E`
  (params (Key :type "Key Structure"))
  ;[1 1 1] Get Off Vehicle
  (:`Pressed`
    (if (`self.isGameNotOver`)
      (if (not (== (`self.Driver`) null))
        (`/Engine/EditorBlueprintResources/ActorMacros.Switch Has Authority`
          (:`Authority`
            (`self.GetOffVehicle` :!label _label)
            (`self.PlayMovingSound` 0.0))
          (:`Remote`
            (`self.GetOffVehicleServer`)))))))

(event `AddMovementServer`
  (params (Axis :type "Float (double-precision)") (deltaTime :type "Float (double-precision)"))
  ;[1 1 1] Add Movement Input
  (`self.UpdateMovement` Axis deltaTime)
  (`self.PlayMovingSound` (`KismetMathLibrary.FMin` (+ (`KismetMathLibrary.Abs` (stale `AddRotateServer` Axis)) (`KismetMathLibrary.Abs` Axis)) 1.0)))

(event `GetOffVehicleServer`
  ;[1 1 1] Get Off Vehicle
  (goto _label))

(event `GetOffVehicle`
  (bind _driver (`self.Driver`))
  ;[1 1 1] Get Off Vehicle
  (`/Engine/EditorBlueprintResources/ActorMacros.Switch Has Authority`
    (:`Authority`
      (`Controller.Possess` (`self.GetController`) _driver)
      (set `/Game/Blueprints/PlayerControllerT.Incar` false _driver)
      (set `self.Driver` null))))

(fn `1/2Angel`
  (bind _outactors (`GameplayStatics.GetAllActorsOfClass` "/Game/Blueprints/EnemyMinion.EnemyMinion_C"))
  (set `self.noneleft` true)
  (for _array_element _outactors
    (if (== (`/Game/Blueprints/EnemyMinion.State` _array_element) 0)
      (set `self.noneleft` false)))
  (if (`self.noneleft`)
    (bind _outactors_2 (`GameplayStatics.GetAllActorsOfClass` "/Script/Engine.AmbientSound"))
    (for _array_element_2 _outactors_2
      (`AudioComponent.Stop` (`AmbientSound.AudioComponent` _array_element_2)))
    (else
      (bind _outactors_3 (`GameplayStatics.GetAllActorsOfClass` "/Script/Engine.AmbientSound"))
      (for _array_element_3 _outactors_3
        (bind _audiocomponent (`AmbientSound.AudioComponent` _array_element_3))
        (if (not (`AudioComponent.IsPlaying` _audiocomponent))
          (`AudioComponent.Play` _audiocomponent 0.0))))))

(fn `AssignDestination`
  (bind _outactors (`GameplayStatics.GetAllActorsOfClass` "/Game/Destination_Blueprint.Destination_Blueprint_C"))
  (for _array_element _outactors
    (set `self.Destination` _array_element)
    (break)))

(fn `ClearUI`
  (bind _foundwidgets (`WidgetBlueprintLibrary.GetAllWidgetsOfClass` "/Game/WinUI.WinUI_C" false))
  (for _array_element _foundwidgets
    (`Widget.RemoveFromParent` _array_element))
  (bind _foundwidgets_2 (`WidgetBlueprintLibrary.GetAllWidgetsOfClass` "/Game/LostUI.LostUI_C" false))
  (for _array_element_2 _foundwidgets_2
    (`Widget.RemoveFromParent` _array_element_2))
  (bind _foundwidgets_3 (`WidgetBlueprintLibrary.GetAllWidgetsOfClass` "/Game/sUI.sUI_C" false))
  (for _array_element_3 _foundwidgets_3
    (`Widget.RemoveFromParent` _array_element_3)))

(fn `IsNearToDes`
  (params (distance :type "Float (double-precision)"))
  (returns (isNear :type Boolean))
  (return (< (`self.GetDistanceTo` (`self.Destination`)) distance)))

(fn `OnHealthZero`
  (`/Engine/EditorBlueprintResources/ActorMacros.Switch Has Authority`
    (:`Authority`
      (`KismetSystemLibrary.PrintString` "Health Reaches 0")
      (set `self.isGameNotOver` false)
      (`self.DisplayLostUI`))))

(fn `OnReachDestination`
  (`/Engine/EditorBlueprintResources/ActorMacros.Switch Has Authority`
    (:`Authority`
      (`KismetSystemLibrary.PrintString` "Reach Destination")
      (set `self.isGameNotOver` false)
      (`self.DisplayWinUI`))))

(fn `RepelPlayer`
  (params (DeltaTime :type "Float (double-precision)") (Axis :type "Float (double-precision)"))
  (bind _returnvalue (`KismetMathLibrary.GetForwardVector` (`KismetMathLibrary.MakeRotator` 0.0 0.0 (.yaw (`self.K2_GetActorRotation`)))))
  (for _array_element (`PrimitiveComponent.GetOverlappingActors` (`self.BlockingTrigger`) "/Game/Blueprints/PlayerControllerT.PlayerControllerT_C")
    (`KismetSystemLibrary.PrintString` (`KismetSystemLibrary.GetDisplayName` _array_element))
    (bind _asplayer_controller_t (cast `/Game/Blueprints/PlayerControllerT` _array_element))
    (if (!= Axis 0.0)
      (`self.K2_AddActorWorldOffset` _array_element (* _returnvalue (* DeltaTime 1500.0 Axis)) false true)
      (`self.K2_AddActorWorldOffset` _asplayer_controller_t (* _returnvalue (* DeltaTime 1500.0 Axis)) false true)
      (else
        (`self.K2_AddActorWorldOffset` _asplayer_controller_t (* _returnvalue (* DeltaTime 1500.0)) false true)))))

(fn `TakeDamage`
  (params (amount :type "Float (double-precision)"))
  (returns (isZero :type Boolean))
  (`/Engine/EditorBlueprintResources/ActorMacros.Switch Has Authority`
    (:`Authority`
      (bind _output_get (set `self.HP` (`KismetMathLibrary.FMax` (- (`self.HP`) amount))))
      (bind _returnvalue (<= _output_get 0.0))
      (if _returnvalue
        (`self.OnHealthZero`))
      (return _returnvalue))))

(fn `UpdateDriverLoc`
  (bind _driver (`self.Driver`))
  (if (not (== _driver null))
    (`self.K2_SetActorLocation` _driver (`self.K2_GetActorLocation` (`self.Spot`)) false true)))

(fn `UpdateMovement`
  (params (Axis :type "Float (double-precision)") (deltaTime :type "Float (double-precision)"))
  (`/Engine/EditorBlueprintResources/ActorMacros.Switch Has Authority`
    (:`Authority`
      (bind _output_get (set `self.Forward` (`KismetMathLibrary.GetForwardVector` (`KismetMathLibrary.MakeRotator` 0.0 0.0 (.yaw (`self.K2_GetActorRotation`))))))
      (bind _output_get_2 (set `self.speedA` (* Axis (`self.speed`) deltaTime)))
      (`self.K2_AddActorWorldOffset` self (* _output_get _output_get_2) true false))))

(fn `UpdateRotation`
  (params (Axis :type "Float (double-precision)") (deltaTime :type "Float (double-precision)"))
  (`/Engine/EditorBlueprintResources/ActorMacros.Switch Has Authority`
    (:`Authority`
      (bind _output_get (set `self.RotateRight` (`KismetMathLibrary.MakeRotator` 0.0 0.0 (* deltaTime Axis 10.0))))
      (`self.K2_AddActorLocalRotation` self _output_get true false))))

(fn `UserConstructionScript`)